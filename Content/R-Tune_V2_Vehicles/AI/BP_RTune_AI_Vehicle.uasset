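; AI-driven R-Tune vehicle pawn that follows a spline, with toggleable interior and free-look cameras.
; Each tick, the RTuneAI component supplies steering, while throttle eases off as angular acceleration rises and cuts during braking.
; Overlapping actors tagged "brakezone" trigger a brief full brake; "endzone" zeroes steering and holds the brakes.
; Brake input also drives the tail-light material parameter.
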(event `InputAction|ToggleFreeCamera`
  (params (Key :type "Key Structure"))
  (bind _springarm (`self.SpringArm`))
  ;[1 1 1] Input
  (:`Pressed`
    (set `SpringArmComponent.bUsePawnControlRotation` (!= (`SpringArmComponent.bUsePawnControlRotation` _springarm) true) _springarm)))

(event `InputAxis|Cx`
  (params (AxisValue :type "Float (single-precision)"))
  ;[1 1 1] Input
  (`self.AddControllerYawInput` AxisValue))

(event `InputAxis|Cy`
  (params (AxisValue :type "Float (single-precision)"))
  ;[1 1 1] Input
  (`self.AddControllerPitchInput` AxisValue))

(event `InputAction|ToggleCamera`
  (params (Key :type "Key Structure"))
  ;[1 1 1] Input
  (:`Pressed`
    (`/Engine/EditorBlueprintResources/StandardMacros.FlipFlop`
      (:`A`
        (`ActorComponent.SetActive` (`self.Camera Interior`) true false)
        (`ActorComponent.SetActive` (`self.Camera`) false false))
      (:`B`
        (`ActorComponent.SetActive` (`self.Camera Interior`) false false)
        (`ActorComponent.SetActive` (`self.Camera`) true false)))))

(event `self.ReceiveBeginPlay`
  ;[1 1 1] Initialize Spline
  (`RTuneAI.SetTargetSpline` (`self.RTuneAI`) (`/Game/R-Tune_V2_Vehicles/AI/BP_Spline.Spline` (`self.Spline`))))

(event `self.ReceiveTick`
  (params (DeltaSeconds :type "Float (single-precision)"))
  (set `self.Delta Time` DeltaSeconds)
  (`|ExecutionSequence`
    (:`then_0`
      (`MeshComponent.SetScalarParameterValueOnMaterials` (`self.CoreMesh`) "Tail Light Input" (`KismetMathLibrary.SelectFloat` 1.0 0.0 (> (`self.GetBrakesInput`) 0.1))))
    (:`then_1`
      ;[1 1 1] AI Update
      (bind _outsteering (`RTuneAI.Update` (`self.RTuneAI`) (`self.Delta Time`)))
      (bind _output_get (set `self.AI Steering` (`KismetMathLibrary.SelectFloat` 0.0 _outsteering (`self.Ended`))))
      (`self.SetSteeringInput` _output_get)
      (bind _output_get_2 (set `self.AI Input` (`KismetMathLibrary.SelectFloat` (`KismetMathLibrary.MapRangeClamped` (`KismetMathLibrary.Abs` (`self.GetAngularAcceleration`)) (`self.Min Angular Acceleration`) (`self.Max Angular Acceleration`) 1.0) 0.0 (== (`self.AI Brakes`) 0.0))))
      (`self.SetThrottleInput` _output_get_2)
      (`self.SetBrakeInput` (`self.AI Brakes`)))))

(event `self.CoreMesh.OnComponentBeginOverlap`
  (params (OverlappedComponent :type "PrimitiveComponent Object Reference") (OtherActor :type "Actor Object Reference") (OtherComp :type "PrimitiveComponent Object Reference") (OtherBodyIndex :type Integer) (bFromSweep :type Boolean) (SweepResult :type "HitResult Structure (by ref)"))
  (bind _tags (`Actor.Tags` OtherActor))
  (bind _output (`|GetArrayItem` _tags))
  ;[1 1 1] Brake Zone Detection
  (if (> (`KismetArrayLibrary.Array_Length` _tags) 0)
    (if (== _output "brakezone")
      (`self.Brake Zone`)
      (elif (== _output "endzone")
        (`self.End Zone`)))))

(event `Brake Zone`
  ;[1 1 1] When the brake zone is detected, apply the brakes for a set amount of time to slowdown
  (set `self.AI Brakes` 1.0)
  (`KismetSystemLibrary.Delay` 0.5)
  (set `self.AI Brakes` 0.0))

(event `End Zone`
  ;[1 1 1] When the end zone is detected, stop
  (set `self.Ended` true)
  (set `self.AI Brakes` 1.0))

(fn `UserConstructionScript`)