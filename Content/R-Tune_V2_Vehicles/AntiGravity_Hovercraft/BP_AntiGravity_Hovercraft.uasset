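; Player-driven anti-gravity hovercraft vehicle Blueprint that passes throttle, brake, steering and air pitch, yaw and roll axes to inherited vehicle setters.
; BeginPlay initializes anti-gravity with the core mesh and a helper scene component.
; Input also drives camera look, toggles spring arm control rotation and switches between interior and exterior cameras.
; Tick updates the speed text and smoothly interpolates thrust material brightness and color from throttle and brake.
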(event `Key|MiddleMouseButton`
  (params (Key :type "Key Structure"))
  (bind _springarm (`self.SpringArm`))
  ;[1 1 1] Input
  (:`Pressed`
    (set `SpringArmComponent.bUsePawnControlRotation` (!= (`SpringArmComponent.bUsePawnControlRotation` _springarm) true) _springarm)))

(event `InputAxis|Air Yaw`
  (params (AxisValue :type "Float (single-precision)"))
  ;[1 1 1] Input
  (`self.SetAirYawInput` AxisValue))

(event `InputAxis|Air Roll`
  (params (AxisValue :type "Float (single-precision)"))
  ;[1 1 1] Input
  (`self.SetAirRollInput` AxisValue))

(event `InputAxis|Cx`
  (params (AxisValue :type "Float (single-precision)"))
  ;[1 1 1] Input
  (`self.AddControllerYawInput` AxisValue))

(event `InputAxis|Brake`
  (params (AxisValue :type "Float (single-precision)"))
  ;[1 1 1] Input
  (`self.SetBrakeInput` AxisValue))

(event `InputAxis|Air Pitch`
  (params (AxisValue :type "Float (single-precision)"))
  ;[1 1 1] Input
  (`self.SetAirPitchInput` AxisValue))

(event `InputAxis|Cy`
  (params (AxisValue :type "Float (single-precision)"))
  ;[1 1 1] Input
  (`self.AddControllerPitchInput` AxisValue))

(event `InputAxis|Throttle`
  (params (AxisValue :type "Float (single-precision)"))
  ;[1 1 1] Input
  (`self.SetThrottleInput` AxisValue))

(event `InputAxis|Steering`
  (params (AxisValue :type "Float (single-precision)"))
  ;[1 1 1] Input
  (`self.SetSteeringInput` AxisValue))

(event `InputAction|ToggleCamera`
  (params (Key :type "Key Structure"))
  ;[1 1 1] Input
  (:`Pressed`
    (`/Engine/EditorBlueprintResources/StandardMacros.FlipFlop`
      (:`A`
        (`ActorComponent.SetActive` (`self.Camera Interior`) true false)
        (`ActorComponent.SetActive` (`self.Camera`) false false))
      (:`B`
        (`ActorComponent.SetActive` (`self.Camera Interior`) false false)
        (`ActorComponent.SetActive` (`self.Camera`) true false)))))

(event `self.ReceiveBeginPlay`
  ;[1 0 0.9333] Anti Gravity Setup
  (`self.InitializeAntiGravity` (`self.AntiGravity`) (`self.Core Mesh`)))

(event `self.ReceiveTick`
  (params (DeltaSeconds :type "Float (single-precision)"))
  (bind _core_mesh (`self.Core Mesh`))
  (bind _returnvalue (`KismetMathLibrary.FClamp` (/ (+ (`self.GetInputAxisValue`) (`self.GetBrakesInput`)) 2.0)))
  ;[1 1 1] Update interior speed text and thrust color
  (set `self.Delta Time` DeltaSeconds)
  (`TextRenderComponent.K2_SetText` (`self.Speed`) (`KismetTextLibrary.Conv_Int64ToText` (`KismetMathLibrary.FFloor64` (`KismetMathLibrary.Abs` (`self.GetSpeedKPH`)))))
  (bind _output_get (set `self.Brightness` (`KismetMathLibrary.FInterpTo` (`self.Brightness`) (`KismetMathLibrary.Lerp` 8.0 150.0 _returnvalue) DeltaSeconds (`KismetMathLibrary.Lerp` 3.0 5.0 _returnvalue))))
  (`MeshComponent.SetScalarParameterValueOnMaterials` _core_mesh "Brightness" _output_get)
  (bind _output_get_2 (set `self.Thrust Color` (`KismetMathLibrary.FInterpTo` (`self.Thrust Color`) (`KismetMathLibrary.SelectFloat` 1.0 0.0 (> (`self.GetBrakesInput`) 0.0)) (`self.Delta Time`) 5.0)))
  (`MeshComponent.SetScalarParameterValueOnMaterials` _core_mesh "Color Switch" _output_get_2))

(fn `UserConstructionScript`
  (`parent.UserConstructionScript`))