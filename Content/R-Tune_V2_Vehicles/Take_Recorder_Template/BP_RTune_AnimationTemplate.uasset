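; R-Tune vehicle pawn template for Take Recorder, drivable with throttle, steering, brake, drift, wheel-lock, burnout and free-camera inputs.
; AsyncTick runs a DriftMode macro that interpolates suspension lateral forces and drift torque between base and handbrake values.
; Tick derives steering limits, wheel spin, burnout, brake lights and camera lag, storing most in Anim variables.
; In RenderMode, Tick instead applies stored wheel-spin, burnout and brake-light values to rear suspensions and materials.
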(event `InputAction|Handbrake`
  (params (Key :type "Key Structure"))
  ;[1 1 1] Input
  (:`Pressed`
    (set `self.Drift Mode` true))
  (:`Released`
    (set `self.Drift Mode` false)))

(event `InputAxis|Throttle`
  (params (AxisValue :type "Float (single-precision)"))
  ;[1 1 1] Input
  (`self.SetThrottleInput` AxisValue))

(event `InputAction|ToggleFreeCamera`
  (params (Key :type "Key Structure"))
  (bind _springarm (`self.SpringArm`))
  (:`Pressed`
    (set `SpringArmComponent.bUsePawnControlRotation` (!= (`SpringArmComponent.bUsePawnControlRotation` _springarm) true) _springarm)))

(event `InputAxis|Steering`
  (params (AxisValue :type "Float (single-precision)"))
  ;[1 1 1] Input
  (`self.SetSteeringInput` AxisValue))

(event `InputAction|Lock Wheels`
  (params (Key :type "Key Structure"))
  ;[1 1 1] Input
  (:`Pressed`
    (set `self.bLock Wheels` true))
  (:`Released`
    (set `self.bLock Wheels` false)))

(event `InputAction|Make Burnout`
  (params (Key :type "Key Structure"))
  ;[1 1 1] Input
  (:`Pressed`
    (set `self.bMakeBurnout` true))
  (:`Released`
    (set `self.bMakeBurnout` false)))

(event `InputAxis|Cx`
  (params (AxisValue :type "Float (single-precision)"))
  (`self.AddControllerYawInput` AxisValue))

(event `InputAxis|Brake`
  (params (AxisValue :type "Float (single-precision)"))
  ;[1 1 1] Input
  (`self.SetBrakeInput` AxisValue))

(event `InputAxis|Cy`
  (params (AxisValue :type "Float (single-precision)"))
  (`self.AddControllerPitchInput` AxisValue))

(event `self.ReceiveBeginPlay`
  ;[1 1 1] Initialize suspension array for DriftMode Macro
  (set `self.Suspension` (`|MakeArray` (`self.Suspension FL`) (`self.Suspension RR`) (`self.Suspension RL`) (`self.Suspension FR`))))

(event `self.AsyncTick`
  (params (DeltaTime :type "Float (single-precision)"))
  (set `self.Async Time` DeltaTime)
  ;[0 0 0] This is an example of how the vehicle behaviour can be extended for more complex and intricate behaviour. The inputs here override their original properties. Then the handbrake is pressed, the new lateral force and drift values, and when it is released the base values are used.
  (`self.DriftMode` 250.0 325.0 3000.0 6500.0 10.0 0.0 4000.0))

(event `self.ReceiveTick`
  (params (DeltaSeconds :type "Float (single-precision)"))
  (set `self.Delta Time` DeltaSeconds)
  (if (`self.Render Mode`)
    (bind _output_get (set `SuspensionComponent.WheelAngularVelocityMultiplier` (`self.Anim Angular Multiplier`) (`self.Suspension RL`)))
    (set `SuspensionComponent.WheelAngularVelocityMultiplier` _output_get (`self.Suspension RR`))
    (bind _output_get_2 (set `SuspensionComponent.BurnoutRotation` (`self.Anim Burnout Rotation`) (`self.Suspension RR`)))
    (set `SuspensionComponent.BurnoutRotation` _output_get_2 (`self.Suspension RL`))
    (`MeshComponent.SetScalarParameterValueOnMaterials` (`self.CoreMesh`) "Tail Light Input" (`self.Anim Brake Lights`))
    (else
      (bind _output_get_3 (set `self.Anim Steering Angle` (`KismetMathLibrary.SelectFloat` (* (`self.Drift Max Angle`) -1.0) (`self.Base Wheel Steer Angle`) (and (`self.Drift Mode`) (> (`self.GetSpeedKPH`) 0.0)))))
      (bind _output_get_4 (set `SuspensionComponent.MaxSteeringAngle` _output_get_3 (`self.Suspension FR`)))
      (set `SuspensionComponent.MaxSteeringAngle` _output_get_4 (`self.Suspension FL`))
      (bind _output_get_5 (set `self.Anim Brake Lights` (`KismetMathLibrary.SelectFloat` 1.0 0.0 (> (`self.GetBrakesInput`) 0.1))))
      (`MeshComponent.SetScalarParameterValueOnMaterials` (`self.CoreMesh`) "Tail Light Input" _output_get_5)
      (bind _output_get_6 (set `self.Anim Angular Multiplier` (`KismetMathLibrary.SelectFloat` 0.0 (`KismetMathLibrary.SelectFloat` (`KismetMathLibrary.Lerp` 1.0 3.0 (`self.GetThrottleInput`)) 1.0 (`self.Drift Mode`)) (`self.bLock Wheels`))))
      (bind _output_get_7 (set `SuspensionComponent.WheelAngularVelocityMultiplier` _output_get_6 (`self.Suspension RL`)))
      (set `SuspensionComponent.WheelAngularVelocityMultiplier` _output_get_7 (`self.Suspension RR`))
      (bind _output_get_8 (set `self.Anim Burnout Rotation` (`KismetMathLibrary.SelectFloat` 5.0 0.0 (`self.bMakeBurnout`))))
      (bind _output_get_9 (set `SuspensionComponent.BurnoutRotation` _output_get_8 (`self.Suspension RL`)))
      (set `SuspensionComponent.BurnoutRotation` _output_get_9 (`self.Suspension RR`))
      (bind _output_get_10 (set `self.Camera Lag` (`KismetMathLibrary.FInterpTo` (`self.Camera Lag`) (`KismetMathLibrary.SelectFloat` 2.0 10.0 (`self.Drift Mode`)) (`self.Delta Time`) 5.0)))
      (set `SpringArmComponent.CameraRotationLagSpeed` _output_get_10 (`self.SpringArm`)))))

(fn `UserConstructionScript`
  (locals (`Approximate Scaling Factor` :type "Float (double-precision)" :default -0.85))
  (`SceneComponent.K2_SetRelativeLocation` (`self.Wheel FR`) (`KismetMathLibrary.MakeVector` 0.0 0.0 (* (`SuspensionComponent.ExtensionLength` (`self.Suspension FR`)) (`local.Approximate Scaling Factor`))) false false)
  (`SceneComponent.K2_SetRelativeLocation` (`self.Wheel RR`) (`KismetMathLibrary.MakeVector` 0.0 0.0 (* (`SuspensionComponent.ExtensionLength` (`self.Suspension RR`)) (`local.Approximate Scaling Factor`))) false false)
  (`SceneComponent.K2_SetRelativeLocation` (`self.Wheel RL`) (`KismetMathLibrary.MakeVector` 0.0 0.0 (* (`SuspensionComponent.ExtensionLength` (`self.Suspension RL`)) (`local.Approximate Scaling Factor`))) false false)
  (`SceneComponent.K2_SetRelativeLocation` (`self.Wheel FL`) (`KismetMathLibrary.MakeVector` 0.0 0.0 (* (`SuspensionComponent.ExtensionLength` (`self.Suspension FL`)) (`local.Approximate Scaling Factor`))) false false))