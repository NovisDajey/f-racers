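; Player-drivable R-Tune V2 vehicle pawn, named as the rear-wheel-drive drivetrain example.
; Input events feed throttle, brake, steering, handbrake and gear shifts, and handle camera look, free-camera and interior/exterior toggles.
; AsyncTick re-couples the decoupled drivetrain RPM during slip, interpolating toward a throttle-scaled maximum through OverrideRPM.
; Tick drives rear-wheel Niagara skidmarks from speed, slip and ground contact, plus a brake-driven tail-light material parameter.
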(event `InputAxis|Throttle`
  (params (AxisValue :type "Float (single-precision)"))
  ;[1 1 1] Input
  (`self.SetThrottleInput` AxisValue))

(event `InputAction|Upshift`
  (params (Key :type "Key Structure"))
  ;[1 1 1] Input
  (:`Pressed`
    (`self.Upshift`)))

(event `InputAction|Upshift`
  (params (Key :type "Key Structure"))
  ;[1 1 1] Input
  (:`Pressed`
    (if (!= (`self.bAutomatic`) true)
      (`self.Upshift`))))

(event `InputAction|Handbrake`
  (params (Key :type "Key Structure"))
  ;[1 1 1] Input
  (:`Pressed`
    (`self.ApplyHandbrakeInput` true))
  (:`Released`
    (`self.ApplyHandbrakeInput` false)))

(event `InputAction|Downshift`
  (params (Key :type "Key Structure"))
  ;[1 1 1] Input
  (:`Pressed`
    (`self.Downshift`)))

(event `InputAxis|Steering`
  (params (AxisValue :type "Float (single-precision)"))
  ;[1 1 1] Input
  (`self.SetSteeringInput` AxisValue))

(event `InputAxis|Brake`
  (params (AxisValue :type "Float (single-precision)"))
  ;[1 1 1] Input
  (`self.SetBrakeInput` AxisValue))

(event `InputAction|Downshift`
  (params (Key :type "Key Structure"))
  ;[1 1 1] Input
  (:`Pressed`
    (if (!= (`self.bAutomatic`) true)
      (`self.Downshift`))))

(event `InputAction|ToggleFreeCamera`
  (params (Key :type "Key Structure"))
  (bind _springarm (`self.SpringArm`))
  ;[1 1 1] Input
  (:`Pressed`
    (set `SpringArmComponent.bUsePawnControlRotation` (!= (`SpringArmComponent.bUsePawnControlRotation` _springarm) true) _springarm)))

(event `InputAction|ToggleCamera`
  (params (Key :type "Key Structure"))
  ;[1 1 1] Input
  (:`Pressed`
    (`/Engine/EditorBlueprintResources/StandardMacros.FlipFlop`
      (:`A`
        (`ActorComponent.SetActive` (`self.Camera Interior`) true false)
        (`ActorComponent.SetActive` (`self.Camera`) false false))
      (:`B`
        (`ActorComponent.SetActive` (`self.Camera Interior`) false false)
        (`ActorComponent.SetActive` (`self.Camera`) true false)))))

(event `InputAxis|Cx`
  (params (AxisValue :type "Float (single-precision)"))
  ;[1 1 1] Input
  (`self.AddControllerYawInput` AxisValue))

(event `InputAxis|Cy`
  (params (AxisValue :type "Float (single-precision)"))
  ;[1 1 1] Input
  (`self.AddControllerPitchInput` AxisValue))

(event `self.AsyncTick`
  (params (DeltaTime :type "Float (single-precision)"))
  ;[1 1 1] Drivetrain RPM is decoupled. This re-couples it so that when the vehicle is slipping, the RPM is 'tied' back
  (if (`self.IsSlipping`)
    (bind _output_get (set `self.RPM` (`KismetMathLibrary.FInterpTo` (`self.RPM`) (* (`self.GetThrottleInput`) (`self.MaxRPM`) 0.95) DeltaTime 5.0)))
    (`self.OverrideRPM` _output_get)
    (else
      (`self.OverrideRPM` (`self.GetRPM`)))))

(event `self.ReceiveTick`
  (params (DeltaSeconds :type "Float (single-precision)"))
  ;[1 1 1] Skidmakrs
  (`NiagaraComponent.SetVariableFloat` (`self.NS_Skid RL`) "SkidRate" (`KismetMathLibrary.SelectFloat` (`KismetMathLibrary.MapRangeClamped` (`KismetMathLibrary.Abs` (`self.GetSpeedKPH`)) 30.0 100.0 200.0 1000.0) 0.0 (and (`self.IsSlipping`) (!= (or (`SuspensionComponent.IsInAir` (`self.Suspension RR`)) (`SuspensionComponent.IsInAir` (`self.Suspension RL`))) true))))
  (`NiagaraComponent.SetVariableFloat` (`self.NS_Skid RR`) "SkidRate" (`KismetMathLibrary.SelectFloat` (`KismetMathLibrary.MapRangeClamped` (`KismetMathLibrary.Abs` (`self.GetSpeedKPH`)) 30.0 100.0 200.0 1000.0) 0.0 (and (`self.IsSlipping`) (!= (or (`SuspensionComponent.IsInAir` (`self.Suspension RR`)) (`SuspensionComponent.IsInAir` (`self.Suspension RL`))) true))))
  (`SceneComponent.K2_SetWorldLocation` (`self.NS_Skid RR`) (`SuspensionComponent.GetOffsetImpactPoint` (`self.Suspension RR`) 3.0) false false)
  (`SceneComponent.K2_SetWorldLocation` (`self.NS_Skid RL`) (`SuspensionComponent.GetOffsetImpactPoint` (`self.Suspension RL`) 3.0) false false)
  (`MeshComponent.SetScalarParameterValueOnMaterials` (`self.CoreMesh`) "Tail Light Input" (`KismetMathLibrary.SelectFloat` 1.0 0.0 (> (`self.GetBrakesInput`) 0.1))))

(fn `UserConstructionScript`)