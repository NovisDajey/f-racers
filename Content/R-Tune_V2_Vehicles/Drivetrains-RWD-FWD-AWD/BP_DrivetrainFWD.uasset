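; Front-wheel-drive example vehicle pawn for R-Tune V2, handling driving input, manual shifting and toggles for interior and free-look cameras.
; Async tick boosts the RPM multiplier during slip and cuts rear suspension lateral force under handbrake so the rear slides.
; Tick drives front-wheel Niagara skid marks from slip, speed and ground contact, and lights tail lamps through a material parameter when braking.
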(event `InputAxis|Cx`
  (params (AxisValue :type "Float (single-precision)"))
  ;[1 1 1] Input
  (`self.AddControllerYawInput` AxisValue))

(event `InputAxis|Throttle`
  (params (AxisValue :type "Float (single-precision)"))
  ;[1 1 1] Input
  (`self.SetThrottleInput` AxisValue))

(event `InputAction|Upshift`
  (params (Key :type "Key Structure"))
  ;[1 1 1] Input
  (:`Pressed`
    (if (!= (`self.bAutomatic`) true)
      (`self.Upshift`))))

(event `InputAction|Handbrake`
  (params (Key :type "Key Structure"))
  ;[1 1 1] Input
  (:`Pressed`
    (`self.ApplyHandbrakeInput` true))
  (:`Released`
    (`self.ApplyHandbrakeInput` false)))

(event `InputAxis|Cy`
  (params (AxisValue :type "Float (single-precision)"))
  ;[1 1 1] Input
  (`self.AddControllerPitchInput` AxisValue))

(event `InputAxis|Steering`
  (params (AxisValue :type "Float (single-precision)"))
  ;[1 1 1] Input
  (`self.SetSteeringInput` AxisValue))

(event `InputAction|Downshift`
  (params (Key :type "Key Structure"))
  ;[1 1 1] Input
  (:`Pressed`
    (if (!= (`self.bAutomatic`) true)
      (`self.Downshift`))))

(event `InputAxis|Brake`
  (params (AxisValue :type "Float (single-precision)"))
  ;[1 1 1] Input
  (`self.SetBrakeInput` AxisValue))

(event `InputAction|ToggleCamera`
  (params (Key :type "Key Structure"))
  ;[1 1 1] Input
  (:`Pressed`
    (`/Engine/EditorBlueprintResources/StandardMacros.FlipFlop`
      (:`A`
        (`ActorComponent.SetActive` (`self.Camera Interior`) true false)
        (`ActorComponent.SetActive` (`self.Camera`) false false))
      (:`B`
        (`ActorComponent.SetActive` (`self.Camera Interior`) false false)
        (`ActorComponent.SetActive` (`self.Camera`) true false)))))

(event `InputAction|ToggleFreeCamera`
  (params (Key :type "Key Structure"))
  (bind _springarm (`self.SpringArm`))
  ;[1 1 1] Input
  (:`Pressed`
    (set `SpringArmComponent.bUsePawnControlRotation` (!= (`SpringArmComponent.bUsePawnControlRotation` _springarm) true) _springarm)))

(event `self.AsyncTick`
  (params (DeltaTime :type "Float (single-precision)"))
  ;[1 1 1] Multiply RPM when slipping
  (set `self.RPM_Multiplier` (`KismetMathLibrary.SelectFloat` 1.3 1.0 (`self.IsSlipping`)))
  ;[1 1 1] Decrease tyre force when handbrake is applied
  (bind _output_get (set `SuspensionComponent.LateralForceScalar` (`KismetMathLibrary.SelectFloat` 1250.0 4520.0 (`self.GetHandbrakeInput`)) (`self.Suspension RL`)))
  (set `SuspensionComponent.LateralForceScalar` _output_get (`self.Suspension RR`)))

(event `self.ReceiveTick`
  (params (DeltaSeconds :type "Float (single-precision)"))
  ;[1 1 1] Skid Makrs
  (`NiagaraComponent.SetVariableFloat` (`self.NS_Skid FR`) "SkidRate" (`KismetMathLibrary.SelectFloat` (`KismetMathLibrary.MapRangeClamped` (`KismetMathLibrary.Abs` (`self.GetSpeedKPH`)) 30.0 100.0 200.0 1000.0) 0.0 (and (`self.IsSlipping`) (!= (or (`SuspensionComponent.IsInAir` (`self.Suspension FR`)) (`SuspensionComponent.IsInAir` (`self.Suspension FL`))) true))))
  (`NiagaraComponent.SetVariableFloat` (`self.NS_Skid FL`) "SkidRate" (`KismetMathLibrary.SelectFloat` (`KismetMathLibrary.MapRangeClamped` (`KismetMathLibrary.Abs` (`self.GetSpeedKPH`)) 30.0 100.0 200.0 1000.0) 0.0 (and (`self.IsSlipping`) (!= (or (`SuspensionComponent.IsInAir` (`self.Suspension FR`)) (`SuspensionComponent.IsInAir` (`self.Suspension FL`))) true))))
  (`SceneComponent.K2_SetWorldLocation` (`self.NS_Skid FR`) (`SuspensionComponent.GetOffsetImpactPoint` (`self.Suspension FR`) 3.0) false false)
  (`SceneComponent.K2_SetWorldLocation` (`self.NS_Skid FL`) (`SuspensionComponent.GetOffsetImpactPoint` (`self.Suspension FL`) 3.0) false false)
  (`MeshComponent.SetScalarParameterValueOnMaterials` (`self.CoreMesh`) "Tail Light Input" (`KismetMathLibrary.SelectFloat` 1.0 0.0 (> (`self.GetBrakesInput`) 0.1))))

(fn `UserConstructionScript`)