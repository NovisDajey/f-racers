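; BP_Excavator is a player-driven excavator vehicle with a controllable arm and bucket.
; Input axes feed throttle, steering and brake, and drive the upper body, three arm segments and bucket through each part's SetInput.
; Actions swap interior and exterior cameras or toggle the spring arm's pawn-control rotation for free look.
; It shows an excavator HUD widget and lights the tail-light material parameter each tick while braking.
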(event `InputAxis|Cx`
  (params (AxisValue :type "Float (single-precision)"))
  ;[1 1 1] Input
  (`self.AddControllerYawInput` (* AxisValue -1.0)))

(event `InputAction|ToggleCamera`
  (params (Key :type "Key Structure"))
  ;[1 1 1] Input
  (:`Pressed`
    (`/Engine/EditorBlueprintResources/StandardMacros.FlipFlop`
      (:`A`
        (`ActorComponent.SetActive` (`self.Camera Interior`) true false)
        (`ActorComponent.SetActive` (`self.Camera`) false false))
      (:`B`
        (`ActorComponent.SetActive` (`self.Camera Interior`) false false)
        (`ActorComponent.SetActive` (`self.Camera`) true false)))))

(event `InputAxis|Cy`
  (params (AxisValue :type "Float (single-precision)"))
  ;[1 1 1] Input
  (`self.AddControllerPitchInput` AxisValue))

(event `InputAxis|Arm Vertical`
  (params (AxisValue :type "Float (single-precision)"))
  ;[1 1 1] Input
  (`ArticulatedComponent.SetInput` (`self.Excavator Upper`) (* AxisValue -1.0)))

(event `InputAxis|Throttle`
  (params (AxisValue :type "Float (single-precision)"))
  ;[1 1 1] Input
  (`self.SetThrottleInput` AxisValue))

(event `InputAxis|Arm 2`
  (params (AxisValue :type "Float (single-precision)"))
  ;[1 1 1] Input
  (`ArticulatedComponent.SetInput` (`self.Arm 1`) (* AxisValue -1.0)))

(event `InputAxis|Steering`
  (params (AxisValue :type "Float (single-precision)"))
  ;[1 1 1] Input
  (`self.SetSteeringInput` AxisValue))

(event `InputAxis|Arm 5`
  (params (AxisValue :type "Float (single-precision)"))
  ;[1 1 1] Input
  (`ArticulatedComponent.SetInput` (`self.Bucket`) AxisValue))

(event `InputAxis|Brake`
  (params (AxisValue :type "Float (single-precision)"))
  ;[1 1 1] Input
  (`self.SetBrakeInput` AxisValue))

(event `InputAxis|Arm 3`
  (params (AxisValue :type "Float (single-precision)"))
  ;[1 1 1] Input
  (`ArticulatedComponent.SetInput` (`self.Arm 2`) AxisValue))

(event `InputAction|ToggleFreeCamera`
  (params (Key :type "Key Structure"))
  (bind _springarm (`self.SpringArm`))
  ;[1 1 1] Input
  (:`Pressed`
    (set `SpringArmComponent.bUsePawnControlRotation` (!= (`SpringArmComponent.bUsePawnControlRotation` _springarm) true) _springarm)))

(event `InputAxis|Arm 4`
  (params (AxisValue :type "Float (single-precision)"))
  ;[1 1 1] Input
  (`ArticulatedComponent.SetInput` (`self.Arm 3`) AxisValue))

(event `self.ReceiveBeginPlay`
  (bind _returnvalue (`|CreateWidget` "/Game/R-Tune_V2_Vehicles/Experimental_Construction_Vehicles/WBP_Excavator.WBP_Excavator_C"))
  (bind _output_get (set `self.Widget` _returnvalue))
  (`UserWidget.AddToViewport` _output_get 0))

(event `self.ReceiveDestroyed`
  (`Widget.RemoveFromParent` (`self.Widget`)))

(event `self.ReceiveTick`
  (params (DeltaSeconds :type "Float (single-precision)"))
  (set `self.Delta Time` DeltaSeconds)
  (`MeshComponent.SetScalarParameterValueOnMaterials` (`self.Core`) "Tail Light Input" (select `bool` (> (`self.GetInputAxisValue`) 0.2) :`true` 1.0 :!type "Float (single-precision)")))

(fn `UserConstructionScript`)