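; BP_Forklift is a drivable forklift vehicle pawn that maps player input to driving, arm and camera controls.
; Axis inputs feed throttle, steering and brake, while inverted Arm Vertical input drives the ForkliftArm component.
; Camera input rotates the view, with toggles for spring arm control rotation and exterior or interior camera.
; Tick drives the Core's tail light material parameter from brake input.
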(event `InputAxis|Cx`
  (params (AxisValue :type "Float (single-precision)"))
  ;[1 1 1] Input
  (`self.AddControllerYawInput` (* AxisValue -1.0)))

(event `Key|MiddleMouseButton`
  (params (Key :type "Key Structure"))
  (bind _springarm (`self.SpringArm`))
  ;[1 1 1] Input
  (:`Pressed`
    (set `SpringArmComponent.bUsePawnControlRotation` (!= (`SpringArmComponent.bUsePawnControlRotation` _springarm) true) _springarm :!label _label)))

(event `InputAxis|Cy`
  (params (AxisValue :type "Float (single-precision)"))
  ;[1 1 1] Input
  (`self.AddControllerPitchInput` AxisValue))

(event `InputAxis|Throttle`
  (params (AxisValue :type "Float (single-precision)"))
  ;[1 1 1] Input
  (`self.SetThrottleInput` AxisValue))

(event `InputAction|ToggleCamera`
  (params (Key :type "Key Structure"))
  ;[1 1 1] Input
  (:`Pressed`
    (`/Engine/EditorBlueprintResources/StandardMacros.FlipFlop`
      (:`A`
        (`ActorComponent.SetActive` (`self.Camera Interior`) true false)
        (`ActorComponent.SetActive` (`self.Camera`) false false))
      (:`B`
        (`ActorComponent.SetActive` (`self.Camera Interior`) false false)
        (`ActorComponent.SetActive` (`self.Camera`) true false)))))

(event `Key|Gamepad_RightThumbstick`
  (params (Key :type "Key Structure"))
  ;[1 1 1] Input
  (:`Pressed`
    (goto _label)))

(event `InputAxis|Steering`
  (params (AxisValue :type "Float (single-precision)"))
  ;[1 1 1] Input
  (`self.SetSteeringInput` AxisValue))

(event `InputAxis|Brake`
  (params (AxisValue :type "Float (single-precision)"))
  ;[1 1 1] Input
  (`self.SetBrakeInput` AxisValue))

(event `InputAxis|Arm Vertical`
  (params (AxisValue :type "Float (single-precision)"))
  ;[1 1 1] Input
  (`ArticulatedComponent.SetInput` (`self.Forklift Arm`) (* AxisValue -1.0)))

(event `self.ReceiveTick`
  (params (DeltaSeconds :type "Float (single-precision)"))
  (set `self.Delta Time` DeltaSeconds)
  (`MeshComponent.SetScalarParameterValueOnMaterials` (`self.Core`) "Tail Light Input" (`KismetMathLibrary.SelectFloat` 1.0 0.0 (> (`self.GetBrakesInput`) 0.1))))

(fn `UserConstructionScript`)