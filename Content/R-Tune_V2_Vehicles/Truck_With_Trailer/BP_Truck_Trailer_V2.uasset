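; Drivable R-Tune V2 truck with a physics-constrained trailer that detaches on F or optionally at start.
; Input events feed throttle, brake, steering, handbrake, manual shifting and a free-look camera toggle.
; TrailerSuspension uses the trailer as its physics body; detaching breaks the constraint and reframes the camera after a delay.
; AsyncTick switches lateral grip on four suspensions with the handbrake, while Tick drives brake-light materials.
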(event `Toggle Free Look`
  (bind _springarm (`self.SpringArm`))
  ;[1 1 1] Input
  (set `SpringArmComponent.bUsePawnControlRotation` (!= (`SpringArmComponent.bUsePawnControlRotation` _springarm) true) _springarm))

(event `InputAction|ToggleFreeCamera`
  (params (Key :type "Key Structure"))
  ;[1 1 1] Input
  (:`Pressed`
    (`self.Toggle Free Look`)))

(event `InputAction|Upshift`
  (params (Key :type "Key Structure"))
  ;[1 1 1] Input
  (:`Pressed`
    (if (!= (`self.bAutomatic`) true)
      (`self.Upshift`))))

(event `InputAxis|Throttle`
  (params (AxisValue :type "Float (single-precision)"))
  ;[1 1 1] Input
  (`self.SetThrottleInput` AxisValue))

(event `InputAxis|Cx`
  (params (AxisValue :type "Float (single-precision)"))
  ;[1 1 1] Input
  (`self.AddControllerYawInput` AxisValue))

(event `InputAction|Downshift`
  (params (Key :type "Key Structure"))
  ;[1 1 1] Input
  (:`Pressed`
    (if (!= (`self.bAutomatic`) true)
      (`self.Downshift`))))

(event `InputAxis|Steering`
  (params (AxisValue :type "Float (single-precision)"))
  ;[1 1 1] Input
  (`self.SetSteeringInput` AxisValue))

(event `InputAxis|Cy`
  (params (AxisValue :type "Float (single-precision)"))
  ;[1 1 1] Input
  (`self.AddControllerPitchInput` AxisValue))

(event `InputAxis|Brake`
  (params (AxisValue :type "Float (single-precision)"))
  ;[1 1 1] Input
  (`self.SetBrakeInput` AxisValue))

(event `InputAction|Handbrake`
  (params (Key :type "Key Structure"))
  ;[1 1 1] Input
  (:`Pressed`
    (`self.ApplyHandbrakeInput` true))
  (:`Released`
    (`self.ApplyHandbrakeInput` false)))

(event `Key|F`
  (params (Key :type "Key Structure"))
  ;[1 1 1] Input
  (:`Pressed`
    (`self.Detach Trailer`)
    (set `self.Trailer Detached` true)))

(event `Detach Trailer`
  (bind (_relative_location_x _relative_location_y _relative_location_z) (`KismetMathLibrary.BreakVector` (`self.Relative Location`)))
  ;[1 1 1] Detach Trailer
  (set `self.Relative Location` (`SceneComponent.RelativeLocation` (`self.SpringArm`)))
  (`PhysicsConstraintComponent.BreakConstraint` (`self.PhysicsConstraint`))
  (`KismetSystemLibrary.Delay` 2.0)
  (`SceneComponent.K2_SetRelativeLocation` (`self.SpringArm`) (`KismetMathLibrary.MakeVector` 0.0 _relative_location_y _relative_location_z) false false)
  (set `SpringArmComponent.TargetArmLength` 1000.0 (`self.SpringArm`)))

(event `self.ReceiveBeginPlay`
  (`SuspensionComponent.SetNewPhysicsBody` (`self.Trailer Suspension`) (`self.Trailer`))
  (if (`self.Break Constraint on Start`)
    (`self.Detach Trailer`)))

(event `self.AsyncTick`
  (params (DeltaTime :type "Float (single-precision)"))
  (for _array_element (`|MakeArray` (`self.SuspensionFR2`) (`self.SuspensionFR1`) (`self.SuspensionFL2`) (`self.SuspensionFL1`))
    ;[1 1 1] Lower traction when handbrake is applied
    (set `SuspensionComponent.LateralForceScalar` (`KismetMathLibrary.SelectFloat` (`self.Rear Tyres Lowered Lateral Force`) (`self.Rear Tyres Base Lateral Force`) (`self.GetHandbrakeInput`)) _array_element)))

(event `self.ReceiveTick`
  (params (DeltaSeconds :type "Float (single-precision)"))
  (bind _trailer (`self.Trailer`))
  (`MeshComponent.SetScalarParameterValueOnMaterials` (`self.Core`) "Tail Light Input" (`KismetMathLibrary.SelectFloat` 1.0 0.0 (> (`self.GetBrakesInput`) 0.1)))
  (if (!= (`self.Trailer Detached`) true)
    (`MeshComponent.SetScalarParameterValueOnMaterials` _trailer "Tail Light Input" (`KismetMathLibrary.SelectFloat` 1.0 0.0 (> (`self.GetBrakesInput`) 0.1)))
    (else
      (`MeshComponent.SetScalarParameterValueOnMaterials` _trailer "Tail Light Input" 0.0))))

(fn `UserConstructionScript`)