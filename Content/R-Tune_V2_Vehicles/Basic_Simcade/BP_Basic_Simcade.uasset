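; Player-driven simcade car pawn built on the R-Tune V2 vehicle system.
; It forwards steering, throttle, brake, handbrake and manual shift input to the vehicle, and handles interior/exterior camera switching plus a free-look toggle.
; Tick drives the tail light material from brake input.
; AsyncTick swaps the rear suspensions' lateral force scalar while the handbrake is held to lower rear traction, overriding their own setting.
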(event `InputAction|ToggleFreeCamera`
  (params (Key :type "Key Structure"))
  (bind _springarm (`self.SpringArm`))
  ;[1 1 1] Input
  (:`Pressed`
    (set `SpringArmComponent.bUsePawnControlRotation` (!= (`SpringArmComponent.bUsePawnControlRotation` _springarm) true) _springarm)))

(event `InputAxis|Cx`
  (params (AxisValue :type "Float (single-precision)"))
  ;[1 1 1] Input
  (`self.AddControllerYawInput` AxisValue))

(event `InputAction|Upshift`
  (params (Key :type "Key Structure"))
  ;[1 1 1] Input
  (:`Pressed`
    (if (!= (`self.bAutomatic`) true)
      (`self.Upshift`))))

(event `InputAxis|Cy`
  (params (AxisValue :type "Float (single-precision)"))
  ;[1 1 1] Input
  (`self.AddControllerPitchInput` AxisValue))

(event `InputAction|Downshift`
  (params (Key :type "Key Structure"))
  ;[1 1 1] Input
  (:`Pressed`
    (if (!= (`self.bAutomatic`) true)
      (`self.Downshift`))))

(event `InputAxis|Steering`
  (params (AxisValue :type "Float (single-precision)"))
  ;[1 1 1] Input
  (`self.SetSteeringInput` AxisValue))

(event `InputAction|ToggleCamera`
  (params (Key :type "Key Structure"))
  ;[1 1 1] Input
  (:`Pressed`
    (`/Engine/EditorBlueprintResources/StandardMacros.FlipFlop`
      (:`A`
        (`ActorComponent.SetActive` (`self.Camera Interior`) true false)
        (`ActorComponent.SetActive` (`self.Camera`) false false))
      (:`B`
        (`ActorComponent.SetActive` (`self.Camera Interior`) false false)
        (`ActorComponent.SetActive` (`self.Camera`) true false)))))

(event `InputAxis|Throttle`
  (params (AxisValue :type "Float (single-precision)"))
  ;[1 1 1] Input
  (`self.SetThrottleInput` AxisValue))

(event `InputAxis|Brake`
  (params (AxisValue :type "Float (single-precision)"))
  ;[1 1 1] Input
  (`self.SetBrakeInput` AxisValue))

(event `InputAction|Handbrake`
  (params (Key :type "Key Structure"))
  ;[1 1 1] Input
  (:`Pressed`
    (`self.ApplyHandbrakeInput` true))
  (:`Released`
    (`self.ApplyHandbrakeInput` false)))

(event `self.ReceiveTick`
  (params (DeltaSeconds :type "Float (single-precision)"))
  (`MeshComponent.SetScalarParameterValueOnMaterials` (`self.CoreMesh`) "Tail Light Input" (`KismetMathLibrary.SelectFloat` 1.0 0.0 (> (`self.GetBrakesInput`) 0.1))))

(event `self.AsyncTick`
  (params (DeltaTime :type "Float (single-precision)"))
  ;[1 1 1] Lower traction when handbrake is applied
  (bind _output_get (set `SuspensionComponent.LateralForceScalar` (`KismetMathLibrary.SelectFloat` (`self.Rear Tyres Lowered Lateral Force`) (`self.Rear Tyres Base Lateral Force`) (`self.GetHandbrakeInput`)) (`self.Suspension RL`)))
  (set `SuspensionComponent.LateralForceScalar` _output_get (`self.Suspension RR`)))

(fn `UserConstructionScript`)