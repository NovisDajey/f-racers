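; BP_Bike_V2 is a drivable bike that feeds steering, throttle, brake and manual gear inputs into inherited vehicle functions.
; It initializes lean steering from the rear suspension and sets stability by sliding four stabilizer components sideways, with an on-screen widget toggled by Y.
; Tick turns the handlebar with front suspension yaw and lights the tail light when braking.
; Inputs also switch interior/exterior cameras and toggle control-rotation orbit against camera lag.
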(event `InputAxis|Steering`
  (params (AxisValue :type "Float (single-precision)"))
  ;[1 1 1] Input
  (`self.SetSteeringInput` AxisValue))

(event `InputAxis|Throttle`
  (params (AxisValue :type "Float (single-precision)"))
  ;[1 1 1] Input
  (`self.SetThrottleInput` AxisValue))

(event `Key|MiddleMouseButton`
  (params (Key :type "Key Structure"))
  (bind _springarm (`self.SpringArm`))
  ;[1 1 1] Input
  (:`Pressed`
    (bind _output_get (set `SpringArmComponent.bUsePawnControlRotation` (!= (`SpringArmComponent.bUsePawnControlRotation` _springarm) true) _springarm))
    (set `SpringArmComponent.bEnableCameraLag` (!= _output_get true) (`self.SpringArm`))))

(event `InputAction|Upshift`
  (params (Key :type "Key Structure"))
  ;[1 1 1] Input
  (:`Pressed`
    (if (!= (`self.bAutomatic`) true)
      (`self.Upshift`))))

(event `InputAxis|Cx`
  (params (AxisValue :type "Float (single-precision)"))
  ;[1 1 1] Input
  (`self.AddControllerYawInput` AxisValue))

(event `InputAxis|Brake`
  (params (AxisValue :type "Float (single-precision)"))
  ;[1 1 1] Input
  (`self.SetBrakeInput` AxisValue))

(event `InputAxis|Cy`
  (params (AxisValue :type "Float (single-precision)"))
  ;[1 1 1] Input
  (`self.AddControllerPitchInput` AxisValue))

(event `InputAction|Downshift`
  (params (Key :type "Key Structure"))
  ;[1 1 1] Input
  (:`Pressed`
    (if (!= (`self.bAutomatic`) true)
      (`self.Downshift`))))

(event `InputAction|ToggleCamera`
  (params (Key :type "Key Structure"))
  ;[1 1 1] Input
  (:`Pressed`
    (`/Engine/EditorBlueprintResources/StandardMacros.FlipFlop`
      (:`A`
        (`ActorComponent.SetActive` (`self.Camera Interior`) true false)
        (`ActorComponent.SetActive` (`self.Camera`) false false))
      (:`B`
        (`ActorComponent.SetActive` (`self.Camera Interior`) false false)
        (`ActorComponent.SetActive` (`self.Camera`) true false)))))

(event `Key|Y`
  (params (Key :type "Key Structure"))
  (bind _stability_widget (`self.Stability Widget`))
  ;[1 1 1] Input
  (:`Pressed`
    (if (`self.Widget Visibility`)
      (`Widget.SetVisibility` _stability_widget "Hidden")
      (set `self.Widget Visibility` false)
      (else
        (`Widget.SetVisibility` _stability_widget "Visible")
        (set `self.Widget Visibility` true)))))

(event `self.ReceiveBeginPlay`
  ;[1 1 1] Required for lean steer. Any suspension component can be used, but it is best to use a rear located component
  (`self.InitializeLeanSteer` (`self.SuspensionRear`))
  ;[1 1 1] Extended functionality for variable stability
  (bind _output_get (set `self.Stabilizers` (`|MakeArray` (`self.StabilizerFront Left`) (`self.StabilizerRear Left`) (`self.StabilizerRear Right`) (`self.StabilizerFront Right`))))
  (for _array_element _output_get
    (`KismetArrayLibrary.Array_Add` (`self.Stabilizer Locations`) (`SceneComponent.RelativeLocation` _array_element)))
  (`self.Set Stability` (`self.Stability`))
  ;[1 0 0] Remove this to remove stability widget UI
  (bind _returnvalue (`|CreateWidget` "/Game/R-Tune_V2_Vehicles/Bikes_V2/WBP_BikeStabilityControls.WBP_BikeStabilityControls_C"))
  (bind _output_get_2 (set `self.Stability Widget` _returnvalue))
  (set `/Game/R-Tune_V2_Vehicles/Bikes_V2/WBP_BikeStabilityControls.Bike` self _output_get_2)
  (`/Game/R-Tune_V2_Vehicles/Bikes_V2/WBP_BikeStabilityControls.Initialize` (`self.Stability Widget`))
  (`UserWidget.AddToViewport` _output_get_2 0))

(event `self.ReceiveDestroyed`
  ;[1 0 0] Remove this to remove stability widget UI
  (`Widget.RemoveFromParent` (`self.Stability Widget`)))

(event `self.ReceiveTick`
  (params (DeltaSeconds :type "Float (single-precision)"))
  (bind (_relativerotation_roll _relativerotation_pitch _relativerotation_yaw) (`KismetMathLibrary.BreakRotator` (`SceneComponent.RelativeRotation` (`self.SuspensionFront`))))
  ;[1 1 1] Animate Front Steering handle bar
  (`SceneComponent.K2_SetRelativeRotation` (`self.SM_Handle`) (`KismetMathLibrary.MakeRotator` 0.0 0.0 _relativerotation_yaw) false false)
  (`MeshComponent.SetScalarParameterValueOnMaterials` (`self.CoreMesh`) "Tail Light Input" (`KismetMathLibrary.SelectFloat` 1.0 0.0 (> (`self.GetBrakesInput`) 0.1))))

(fn `Set Stability`
  (params (Stability :type "Float (double-precision)"))
  (for (_array_element _array_index) (`self.Stabilizers`)
    (`SceneComponent.K2_SetRelativeLocation` _array_element (`KismetMathLibrary.MakeVector` (.x (`|GetArrayItem` (`self.Stabilizer Locations`) _array_index)) (* Stability 20.0 (`KismetMathLibrary.SelectFloat` 1.0 -1.0 (> _array_index 1))) (.z (`|GetArrayItem` (`self.Stabilizer Locations`) _array_index))) false false)))

(fn `UserConstructionScript`)